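; BP_Pawn is a duck board game piece that advances along the board one tile per MovePawn press.
; BeginPlay picks the duck mesh's material from its Color value.
; Each press increments CurrentTile up to a hard-coded last index, then teleports the pawn to that tile actor's location and rotation from the BoardTiles array.
; An IsPawnMoving flag guards the move but clears immediately, as the teleport is instant.
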(event EventBeginPlay
  (bind _duck (Variables|Default|Getduck))
  (switch string (Variables|Default|Getcolor)
    (:Default
      (Rendering|Material|SetMaterial _duck 0 "/Game/Meshes/duck_Material.duck_Material"))
    (:Red
      (Rendering|Material|SetMaterial _duck 0 "/Game/Meshes/duck_MaterialRed.duck_MaterialRed"))
    (:Blue
      (Rendering|Material|SetMaterial _duck 0 "/Game/Meshes/duck_MaterialBlue.duck_MaterialBlue"))
    (:Green
      (Rendering|Material|SetMaterial _duck 0 "/Game/Meshes/duck_MaterialGreen.duck_MaterialGreen"))
    (:Orange
      (Rendering|Material|SetMaterial _duck 0 "/Game/Meshes/duck_MaterialOrange.duck_MaterialOrange"))
    (:Black
      (Rendering|Material|SetMaterial _duck 0 "/Game/Meshes/duck_MaterialBlack.duck_MaterialBlack"))))

(event Input|ActionEvents|InputActionMovePawn
  (params (Key :type Key%20Structure :default "None"))
  (:Pressed
    (if (not (Variables|Default|GetisPawnMoving))
      (if (not (>= (Variables|Default|GetcurrentTile) 69))
        (Variables|Default|SetisPawnMoving true)
        (bind _result (Math|Integer|IncrementInt (Variables|Default|GetcurrentTile))
          (:%20%20
            (bind _output_get (Variables|Default|SetcurrentTile _result))
            (Transformation|SetActorLocationAndRotation (Transformation|GetActorLocation (Utilities|Array|Get(acopy) (Variables|/Game/Blueprint/BP_BoardTiles.BP_BoardTiles_C|GetBoardTiles (Variables|Default|GetboardTiles)) _output_get)) (Transformation|GetActorRotation (Utilities|Array|Get(acopy) (Variables|/Game/Blueprint/BP_BoardTiles.BP_BoardTiles_C|GetBoardTiles (Variables|Default|GetboardTiles)) _output_get)) false true)
            (Variables|Default|SetisPawnMoving false)))))))

(fn ConstructionScript)